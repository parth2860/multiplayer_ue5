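; Demo Game Instance that handles PlayFab accounts and multiplayer matchmaking.
; Init applies title settings; Register and Login store player identity, which StartMatchmaking uses to create a ticket behind a DoOnce.
; A looping timer polls the ticket until matched, then GetMatch supplies the server IP and port for an Open console command.
; Separate events cover session host/join, a CloudScript hosted flag and queue statistics; GSDK server registration is left unwired.
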(event Custom|reset%20matchmaking
  (bind _returnvalue (Class|PlayFabJsonObject|ConstructJsonObject))
  ;[1 1 1] create match making ticket
  (Utilities|FlowControl|DoOnce false) ; enters at Reset
)

(event Custom|act_success
  (params (result :type Client%20Register%20Play%20Fab%20User%20Result%20Structure) (customData :type Object%20Object%20Reference))
  (bind (_entitytoken _playfabid) (Utilities|Struct|BreakClientRegisterPlayFabUserResult result))
  ;[1 1 1] register and login
  (Variables|Default|SetEntity%20token _entitytoken)
  (Variables|Default|SetPlay%20Fab%20Id _playfabid)
  (Development|PrintString "account registered"))

(event Custom|get%20matchmaking%20ticket%20fail
  (params (error :type Play%20Fab%20Error%20Structure) (customData :type Object%20Object%20Reference))
  ;[1 1 1] get matchmaking ticket
  (Development|PrintString "get match making ticket fail"))

(event Custom|Get%20AccountInfo
  (|GetAccountInfo (Utilities|Struct|MakeClientGetAccountInfoRequest (Variables|Default|GetPlay%20Fab%20Id)) (delegate Custom|SuccessAccountInfo) (delegate Custom|CustomEvent_1)))

(event Custom|SuccessAccountInfo
  (params (result :type Client%20Get%20Account%20Info%20Result%20Structure) (customData :type Object%20Object%20Reference))
  (Utilities|FlowControl|Sequence
    (:then_0
      (Development|PrintString (Utilities|String|Append "Player ID is: " (Class|PlayFabJsonObject|GetStringField (Class|PlayFabJsonObject|GetObjectField (Class|PlayFabJsonObject|GetObjectField (.AccountInfo (Utilities|Struct|BreakClientGetAccountInfoResult result)) "TitleInfo") "TitlePlayerAccount") "Id"))))
    (:then_1)))

(event Custom|find%20match%20timer
  ;[1 1 1] create match making ticket
  (CallFunction|GetMatchmakingTicket)
  (Development|PrintString "ticket created"))

(event Custom|get%20matchmaking%20ticket
  ;[1 1 1] get matchmaking ticket
  (|GetMatchmakingTicket (Utilities|Struct|MakeMultiplayerGetMatchmakingTicketRequest 0 false (Variables|Default|GetQueue%20Name) (Variables|Default|GetTicket%20Id)) (delegate Custom|get%20matchmaking%20success) (delegate Custom|get%20matchmaking%20ticket%20fail)))

(event Custom|matchmaking%20success%20created
  (params (result :type Multiplayer%20Create%20Matchmaking%20Ticket%20Result%20Structure) (customData :type Object%20Object%20Reference))
  ;[1 1 1] create match making ticket
  (Variables|Default|SetTicket%20Id (.TicketId (Utilities|Struct|BreakMultiplayerCreateMatchmakingTicketResult result)))
  (bind _returnvalue (Utilities|Time|SetTimerbyEvent (delegate Custom|find%20match%20timer) 1e+01 true))
  (Variables|Default|Setmatch%20making%20timer%20handler _returnvalue))

(event Custom|GetQueueStatistics
  ;[1 1 1] For UI if you need to show how much players connected for example,only work wirh dedicated server
  (|GetQueueStatistics (Utilities|Struct|MakeMultiplayerGetQueueStatisticsRequest 0 (Variables|Default|GetQueue%20Name)) (delegate Custom|SuccassQueueStatistics) (delegate Custom|fail%20queue%20statistics)))

(event Custom|SuccassQueueStatistics
  (params (result :type Multiplayer%20Get%20Queue%20Statistics%20Result%20Structure) (customData :type Object%20Object%20Reference))
  ;[1 1 1] For UI if you need to show how much players connected for example,only work wirh dedicated server
  (Development|PrintString (Utilities|String|ToString(Float) (Class|PlayFabJsonValue|AsNumber (Class|PlayFabJsonObject|GetField (.TimeToMatchStatisticsInSeconds (Utilities|Struct|BreakMultiplayerGetQueueStatisticsResult result)) "Average")))))

(event Custom|leaderboard
  (|GetLeaderboard (Utilities|Struct|MakeLeaderboardsGetEntityLeaderboardRequest)))

(event Custom|CustomEvent_1
  (params (error :type Play%20Fab%20Error%20Structure) (customData :type Object%20Object%20Reference))
  (Development|PrintString "matchmaking ticket creation fail"))

(event Custom|get%20match%20making
  ;[1 1 1] get match request
  (|GetMatch (Utilities|Struct|MakeMultiplayerGetMatchRequest 0 false (Variables|Default|GetMatch%20Id) (Variables|Default|GetQueue%20Name) true) (delegate Custom|get%20match%20success) (delegate Custom|get%20match%20fail)))

(event Custom|player_matchmaking
  ;[1 1 1] create match making ticket
)

(event Custom|create%20matchmaking%20ticket%20fail
  (params (error :type Play%20Fab%20Error%20Structure) (customData :type Object%20Object%20Reference))
  ;[1 1 1] create match making ticket
  (Development|PrintString "matchmaking ticket creation fail")
  (Utilities|FlowControl|Delay 5.0)
  (CallFunction|ResetMatchmaking))

(event Custom|fail%20queue%20statistics
  (params (error :type Play%20Fab%20Error%20Structure) (customData :type Object%20Object%20Reference))
  ;[1 1 1] For UI if you need to show how much players connected for example,only work wirh dedicated server
  (Development|PrintString (.ErrorMessage (Utilities|Struct|BreakPlayFabError error))))

(event Custom|validate%20token
  (|ValidateEntityToken (Utilities|Struct|MakeAuthenticationValidateEntityTokenRequest 0 (Utilities|GetDisplayName (Variables|Default|GetEntity%20token))) 0 (delegate Custom|validation%20failed)))

(event Custom|chess%20timer
  (bind _output_get (Variables|Default|Setvalue (+ (Variables|Default|Getvalue) 1.0)))
  (if (>= _output_get 1.2e+02)
    (CallFunction|ChessTimer)
    (else
      (Variables|Default|Setvalue 0.0))))

(event Custom|validation%20failed
  (params (error :type Play%20Fab%20Error%20Structure) (customData :type Object%20Object%20Reference))
  (Development|PrintString (.ErrorMessage (Utilities|Struct|BreakPlayFabError error)))
  (Development|PrintString "validation fail"))

(event Custom|host%20session
  ;[1 1 1] local session
  (|Session (Game|GetPlayerController 0) 5 false false
    (:OnSuccess
      (Development|PrintString "session created")
      (Game|OpenLevel(byName) "demo_spawn" true "?listen"))
    (:OnFailure
      (Development|PrintString "session did not created"))))

(event Custom|join%20session
  (bind _returnvalue (Game|GetPlayerController 0))
  ;[1 1 1] local session
  (bind _results (|FindSessions _returnvalue 10 false)
    (:OnSuccess
      (|JoinSession _returnvalue (Utilities|Array|Get(acopy) _results)
        (:OnSuccess
          (Development|PrintString " session joined"))
        (:OnFailure
          (Development|PrintString "session join failed"))))))

(event Custom|CustomEvent_2
  (params (result :type Client%20Execute%20Cloud%20Script%20Result%20Structure) (customData :type Object%20Object%20Reference))
  ;[1 1 1] value updated on server as well
  (Development|PrintString (.ErrorMessage (Utilities|Struct|BreakPlayFabError (stale Custom|CustomEvent_3 error)))))

(event Custom|CustomEvent_3
  (params (error :type Play%20Fab%20Error%20Structure) (customData :type Object%20Object%20Reference))
  ;[1 1 1] value updated on server as well
  (Development|PrintString (.ErrorMessage (Utilities|Struct|BreakPlayFabError error))))

(event Custom|CustomEvent
  (params (error :type Play%20Fab%20Error%20Structure) (customData :type Object%20Object%20Reference))
  ;[1 1 1] register and login
  (Development|PrintString (.ErrorMessage (Utilities|Struct|BreakPlayFabError error))))

(event Custom|dataupdate_succes
  (params (result :type Client%20Execute%20Cloud%20Script%20Result%20Structure) (customData :type Object%20Object%20Reference))
  ;[1 1 1] nor mal valur get and receive
  (Development|PrintString (.ErrorMessage (Utilities|Struct|BreakPlayFabError (stale Custom|dataupdate_fail error)))))

(event Custom|dataupdate_fail
  (params (error :type Play%20Fab%20Error%20Structure) (customData :type Object%20Object%20Reference))
  ;[1 1 1] nor mal valur get and receive
  (Development|PrintString (.ErrorMessage (Utilities|Struct|BreakPlayFabError error))))

(event Custom|register%20gsdk_shutdown_delegate
  ;[1 1 1] event init
  (Game|QuitGame 0 "Quit" false))

(event Custom|register%20gsdk%20maintenance
  (params (MaintenanceSchedule :type Maintenance%20Schedule%20Structure%20%28by%20ref%29))
  ;[1 1 1] event init
)

(event Custom|get%20session_confirmation
  ;[1 1 1] value updated on server as well
  (bind _response (|ExecuteCloudScript (Utilities|Struct|MakeClientExecuteCloudScriptRequest 0 "updateIsHosted" (Variables|Default|GetFunction%20Parameter)) (delegate Custom|CustomEvent_2) (delegate Custom|CustomEvent_3))
    (:OnPlayFabResponse
      (Development|PrintString (Class|PlayFabJsonObject|GetStringField (Class|PlayFabJsonObject|GetObjectField (.responseData (Utilities|Struct|BreakPlayFabBaseModel _response)) "Data") "FunctionName"))
      (Development|PrintString (Utilities|String|ToString(Boolean) (Class|PlayFabJsonObject|GetBoolField (Class|PlayFabJsonObject|GetObjectField (Class|PlayFabJsonObject|GetObjectField (.responseData (Utilities|Struct|BreakPlayFabBaseModel _response)) "Data") "FunctionResult") "IsHosted")))
      (Variables|Default|Setsession%20hosted? (Class|PlayFabJsonObject|GetBoolField (Class|PlayFabJsonObject|GetObjectField (Class|PlayFabJsonObject|GetObjectField (.responseData (Utilities|Struct|BreakPlayFabBaseModel _response)) "Data") "FunctionResult") "IsHosted")))))

(event Custom|destroy%20session
  ;[1 1 1] local session
  (bind _results (|FindSessions (Game|GetPlayerController 0) 10 false)))

(event Custom|register%20active%20delegates
  ;[1 1 1] event init
)

(event Custom|register_ready%20for%20player
  ;[1 1 1] event init
)

(event Custom|login_succes
  (params (result :type Client%20Login%20Result%20Structure) (customData :type Object%20Object%20Reference))
  (bind (_entitytoken _inforesultpayload _lastlogintime _newlycreated _playfabid) (Utilities|Struct|BreakClientLoginResult result))
  (bind _returnvalue (Class|PlayFabJsonObject|GetObjectField _entitytoken "Entity"))
  (bind _returnvalue_2 (Class|PlayFabJsonObject|GetStringField _returnvalue "Id"))
  ;[1 1 1] register and login
  (bind _output_get (Variables|Default|SetEntity%20token _entitytoken))
  (bind _output_get_2 (Variables|Default|SetPlay%20Fab%20Id _playfabid))
  (Development|PrintString "user login")
  (Development|PrintString _returnvalue_2)
  (Variables|Default|Setentity_id _returnvalue_2))

(event Custom|login_fail
  (params (error :type Play%20Fab%20Error%20Structure) (customData :type Object%20Object%20Reference))
  ;[1 1 1] register and login
  (Development|PrintString (.ErrorMessage (Utilities|Struct|BreakPlayFabError error))))

(event Custom|get%20matchmaking%20success
  (params (result :type Multiplayer%20Get%20Matchmaking%20Ticket%20Result%20Structure) (customData :type Object%20Object%20Reference))
  (bind (_cancellationreasonstring _changenumber _created _creator _giveupafterseconds _matchid _members _memberstomatchwith _queuename _status) (Utilities|Struct|BreakMultiplayerGetMatchmakingTicketResult result))
  ;[1 1 1] get matchmaking ticket
  (Variables|Default|SetMatch%20Id _matchid)
  (Variables|Default|SetStatus _status)
  (if (Utilities|Enum|Equal(Enum) _status "matched")
    (Utilities|Time|ClearandInvalidateTimerbyHandle (Variables|Default|Getmatch%20making%20timer%20handler))
    (CallFunction|GetMatchMaking)
    (Development|PrintString "getting matchmaking  ticket succed")))

(event Custom|get%20match%20success
  (params (result :type Multiplayer%20Get%20Match%20Result%20Structure) (customData :type Object%20Object%20Reference))
  (bind (_arrangementstring _matchid _members _regionpreferences _serverdetails) (Utilities|Struct|BreakMultiplayerGetMatchResult result))
  ;[1 1 1] get match request
  (if (Utilities|Enum|Equal(Enum) _matchid (Variables|Default|GetMatch%20Id))
    ;;[0 1 0.9889] playfab_dedicated server
    (bind _returnvalue (Class|PlayFabJsonObject|GetObjectArrayField _serverdetails "Ports"))
    (Development|ExecuteConsoleCommand (Utilities|String|Append "Open" (Class|PlayFabJsonValue|AsString (Class|PlayFabJsonObject|GetField _serverdetails "IPv4Address")) " / " (Utilities|String|ToString(Float) (Class|PlayFabJsonObject|GetNumberField (Utilities|Array|Get(acopy) _returnvalue) "Num"))) 0)))

(event Custom|get%20entity%20token)

(event Custom|get%20match%20fail
  (params (error :type Play%20Fab%20Error%20Structure) (customData :type Object%20Object%20Reference))
  ;[1 1 1] get match request
  (Development|PrintString "fail to get match"))

(event EventStartMatchmaking
  (bind _returnvalue (Class|PlayFabJsonObject|ConstructJsonObject))
  ;[1 1 1] create match making ticket
  (Utilities|FlowControl|DoOnce false
    (:Completed
      (Variables|Default|Setcreater%20setting _returnvalue)
      (Variables|Default|SetEntity%20token _returnvalue)
      (Variables|Default|Setlatencies _returnvalue)
      (Variables|Default|SetlatencyItem _returnvalue)
      (Variables|Default|SetAttributes _returnvalue)
      (Class|PlayFabJsonObject|SetStringField (Variables|Default|GetlatencyItem) "region" "EastAsia")
      (Class|PlayFabJsonObject|SetStringField (Variables|Default|GetlatencyItem) "latencies" "150")
      (Class|PlayFabJsonObject|SetArrayField (Variables|Default|Getlatencies) "Latencies" (Utilities|Array|MakeArray (Class|PlayFabJsonValue|ConstructJsonValueObject (Variables|Default|GetlatencyItem))))
      (Class|PlayFabJsonObject|SetStringField (Variables|Default|GetEntity%20token) "Id" (Variables|Default|Getentity_id))
      (Class|PlayFabJsonObject|SetStringField (Variables|Default|GetEntity%20token) "Type" "title_player_account")
      (Class|PlayFabJsonObject|SetStringField (Variables|Default|GetEntity%20token) "TypeString" "title_player_account")
      (Class|PlayFabJsonObject|SetObjectField (Variables|Default|GetAttributes) "DataObject" (Variables|Default|Getlatencies))
      (Class|PlayFabJsonObject|SetObjectField (Variables|Default|Getcreater%20setting) "Attributes" (Variables|Default|GetAttributes))
      (Class|PlayFabJsonObject|SetObjectField (Variables|Default|Getcreater%20setting) "Entity" (Variables|Default|GetEntity%20token))
      (|MatchmakingTicket (Utilities|Struct|MakeMultiplayerCreateMatchmakingTicketRequest (Variables|Default|Getcreater%20setting) 0 120 0 (Variables|Default|GetQueue%20Name)) (delegate Custom|matchmaking%20success%20created) (delegate Custom|create%20matchmaking%20ticket%20fail)))))

(event EventRunscript
  ;[1 1 1] value updated on server as well
  (bind _response (|ExecuteCloudScript (Utilities|Struct|MakeClientExecuteCloudScriptRequest 0 "updateIsHosted" (Variables|Default|GetFunction%20Parameter)) (delegate Custom|CustomEvent_2) (delegate Custom|CustomEvent_3))
    (:OnPlayFabResponse
      (Development|PrintString (Class|PlayFabJsonObject|GetStringField (Class|PlayFabJsonObject|GetObjectField (.responseData (Utilities|Struct|BreakPlayFabBaseModel _response)) "Data") "FunctionName"))
      (Development|PrintString (Utilities|String|ToString(Boolean) (Class|PlayFabJsonObject|GetBoolField (Class|PlayFabJsonObject|GetObjectField (Class|PlayFabJsonObject|GetObjectField (.responseData (Utilities|Struct|BreakPlayFabBaseModel _response)) "Data") "FunctionResult") "IsHosted")))
      (Variables|Default|Setsession%20hosted? (Class|PlayFabJsonObject|GetBoolField (Class|PlayFabJsonObject|GetObjectField (Class|PlayFabJsonObject|GetObjectField (.responseData (Utilities|Struct|BreakPlayFabBaseModel _response)) "Data") "FunctionResult") "IsHosted")))))

(event EventRegister
  (params (username :type String) (email :type String) (password :type String))
  ;[1 1 1] register and login
  (|RegisterPlayFabUser (Utilities|Struct|MakeClientRegisterPlayFabUserRequest 0 username email "" 0 password "" false username) (delegate Custom|act_success) (delegate Custom|CustomEvent)))

(event EventLogin
  (params (username :type String) (email :type String) (password :type String))
  ;[1 1 1] register and login
  (|LoginwithPlayFab (Utilities|Struct|MakeClientLoginWithPlayFabRequest 0 0 password username) (delegate Custom|login_succes) (delegate Custom|login_fail)))

(event EventInit
  ;[1 1 1] event init
  (Class|PlayFabUtilities|SetPlayFabSettings (Variables|Default|GetGame%20Title%20Id) (Variables|Default|GetPlay%20Fab%20Secret%20Api%20Key)))

(fn BpGiDemoAutoGenFunc
  (return false))

(fn GetMatchmakingStatus
  (return ""))